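; BP_Player is the player character Blueprint, declaring a targeting API that is not yet implemented.
; Its functions cover getting and setting a target and targeter, checking targeting state, and focusing the view on a target.
; All are stubs returning false or nothing, the event nodes are disabled, and the construction script only calls its parent.
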(event EventBeginPlay)

(event EventActorBeginOverlap
  (params (OtherActor :type Actor%20Object%20Reference)))

(event EventTick
  (params (DeltaSeconds :type Float%20%28single-precision%29)))

(fn ConstructionScript
  (|CallParentFunction))

(fn FocusViewonTarget
  (params (CurrentTarget :type BPI%20Targetable%20Interface))
  (return false))

(fn GetIsTargeted
  (return false))

(fn GetIsTargeting
  (return false))

(fn GetTarget
  (return 0))

(fn GetTargeter
  (return 0))

(fn SetTarget
  (params (NewTarget :type BPI%20Targetable%20Interface) (Nullify :type Boolean))
  (return 0))

(fn SetTargeter
  (params (NewTargeter :type BPI%20Targeter%20Interface))
  (return 0))