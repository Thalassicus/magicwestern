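; BP_TargetingSystem is a prototype component that outlines an interface for tracking a target and a targeter.
; It declares getters and setters for both, plus queries for targeting and targeted state, but these are stubs returning false.
; SetTargeter ignores its input and clears MyTargeter, SetTarget stores nothing, and the Tick and InitializeComponent events are disabled.
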(event EventTick
  (params (DeltaSeconds :type Float%20%28single-precision%29)))

(event EventInitializeComponent)

(fn GetIsTargeted
  (return false))

(fn GetIsTargeting
  (return false))

(fn GetTarget
  (return false))

(fn GetTargeter
  (return false))

(fn SetTarget
  (params (NewTarget :type Boolean))
  (return false))

(fn SetTargeter
  (params (NewTargeter :type Boolean))
  (Variables|TargetingObjects|SetMyTargeter 0)
  (return false))