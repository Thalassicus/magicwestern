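; BP_PDPlayerController is a player controller that moves the controlled pawn relative to the camera.
; The MoveForward and MoveRight axis events feed movement input along forward and right vectors built from the camera manager's yaw, ignoring pitch and roll.
; Disconnected nodes retain older pawn-yaw and absolute-north variants for reference, and BeginPlay, Tick and the construction script are empty.
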(event EventBeginPlay)

(event EventTick
  (params (DeltaSeconds :type Float%20%28single-precision%29)))

(event Input|AxisEvents|InputAxisMoveRight
  (params (AxisValue :type Float%20%28single-precision%29))
  (Pawn|Input|AddMovementInput (Pawn|GetControlledPawn) (Math|Vector|GetRightVector (Class|KismetMathLibrary|MakeRot 0.0 (.Yaw (Class|KismetMathLibrary|BreakRot (Camera|GetCameraRotation (Game|GetPlayerCameraManager 0)))) 0.0)) AxisValue false))

(event Input|AxisEvents|InputAxisMoveForward
  (params (AxisValue :type Float%20%28single-precision%29))
  (Pawn|Input|AddMovementInput (Pawn|GetControlledPawn) (Math|Vector|GetForwardVector (Class|KismetMathLibrary|MakeRot 0.0 (.Yaw (Class|KismetMathLibrary|BreakRot (Camera|GetCameraRotation (Game|GetPlayerCameraManager 0)))) 0.0)) AxisValue false))

(fn ConstructionScript)