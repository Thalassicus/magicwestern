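; BP_PDGameInstance is the prototype's game instance, which sets up the skill library, player arsenal and save game on Init.
; It spawns and initializes a BP_SkillLibrary actor, then creates a new BP_PDSaveGame with a hardcoded player name.
; It spawns a BP_SkillArsenal if none is valid, then writes the new save to its own slot without loading any existing one.
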(event EventInit
  (bind _returnvalue (Game|SpawnActorfromClass "/Game/PrototypeContent/Blueprints/Actors/BP_SkillLibrary.BP_SkillLibrary_C" (Variables|Default|GetSkillLibrarySpawnPoint) false 0 0 0))
  (bind _output_get (Variables|Default|SetSkillLibrary _returnvalue))
  (Default|Initialize _output_get)
  (bind _returnvalue_2 (SaveGame|CreateSaveGameObject))
  (bind _asbp_pdsave_game (Utilities|Casting|CastToBP_PDSaveGame _returnvalue_2))
  (bind _output_get_2 (Variables|Default|SetOmni_SaveGame _asbp_pdsave_game))
  (Variables|/Game/PrototypeContent/Blueprints/GameData/BP_PDSaveGame.BP_PDSaveGame_C|SetPlayerName _output_get_2 "PlayerOne")
  (Utilities|IsValid (Variables|Default|GetPlayerArsenal)
    (:Is%20Valid
      _)
    (:Is%20Not%20Valid
      (bind _returnvalue_3 (Game|SpawnActorfromClass "/Game/PrototypeContent/Blueprints/Actors/BP_SkillArsenal.BP_SkillArsenal_C" (Math|Transform|MakeTransform "0, 0, 0") false 0))
      (Variables|Default|SetPlayerArsenal _returnvalue_3)))
  (SaveGame|SaveGametoSlot (Variables|Default|GetOmni_SaveGame) (Variables|/Game/PrototypeContent/Blueprints/GameData/BP_PDSaveGame.BP_PDSaveGame_C|GetSaveSlotName (Variables|Default|GetOmni_SaveGame)) (Variables|/Game/PrototypeContent/Blueprints/GameData/BP_PDSaveGame.BP_PDSaveGame_C|GetUserIndex (Variables|Default|GetOmni_SaveGame))))