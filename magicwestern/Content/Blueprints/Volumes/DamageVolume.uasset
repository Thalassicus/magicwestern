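; DamageVolume is a volume actor that deals periodic damage to actors overlapping it.
; Begin and end overlap events maintain a unique list of those actors, with no filtering by type.
; Tick accumulates time and, once past Interval, damages each listed actor by DamagePerSecond times Interval, with itself as damage causer.
; The timer carries its remainder forward, but applies at most one pulse per frame.
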(event EventActorBeginOverlap
  (params (OtherActor :type Actor%20Object%20Reference))
  (Utilities|Array|AddUnique (Variables|Default|GetActorCollisions) OtherActor))

(event EventTick
  (params (DeltaSeconds :type Float%20%28single-precision%29))
  (if (> (+ DeltaSeconds (Variables|Default|GetTimer)) (Variables|Default|GetInterval))
    (Variables|Default|SetTimer (- (+ DeltaSeconds (Variables|Default|GetTimer)) (Variables|Default|GetInterval)))
    (for _array_element (Variables|Default|GetActorCollisions)
      (Game|Damage|ApplyDamage _array_element (* (Variables|Default|GetDamagePerSecond) (Variables|Default|GetInterval)) 0 self))
    (else
      (Variables|Default|SetTimer (+ DeltaSeconds (Variables|Default|GetTimer))))))

(event EventActorEndOverlap
  (params (OtherActor :type Actor%20Object%20Reference))
  (Utilities|Array|RemoveItem (Variables|Default|GetActorCollisions) OtherActor))

(fn ConstructionScript)