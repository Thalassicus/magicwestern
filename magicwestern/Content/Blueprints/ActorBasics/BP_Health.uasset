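; BP_Health is a health Blueprint that tracks current and maximum health and exposes functions for damage, healing and queries.
; Damage and healing clamp CurrentHealth between zero and MaximumHealth, returning whether health remains above zero or below maximum, respectively.
; GetHealth returns both values.
; DoDeath, GetIsAlive and SetCurrentHealth are stubs that return constant false or zero without changing state.
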(fn DoDeath
  (return false))

(fn GetHealth
  (return (Variables|Default|GetCurrentHealth) (Variables|Default|GetMaximumHealth)))

(fn GetIsAlive
  (return false))

(fn OnTakeDamage
  (params (Damage%20Amount :type Float%20%28single-precision%29))
  (Variables|Default|SetCurrentHealth (Math|Float|Clamp(Float) (- (Variables|Default|GetCurrentHealth) Damage%20Amount) 0.0 (Variables|Default|GetMaximumHealth)))
  (return (> (Variables|Default|GetCurrentHealth) 0.0)))

(fn OnTakeHeal
  (params (Heal%20Amount :type Float%20%28single-precision%29))
  (bind _maximumhealth (Variables|Default|GetMaximumHealth))
  (Variables|Default|SetCurrentHealth (Math|Float|Clamp(Float) (+ Heal%20Amount (Variables|Default|GetCurrentHealth)) 0.0 _maximumhealth))
  (return (> _maximumhealth (Variables|Default|GetCurrentHealth))))

(fn SetCurrentHealth
  (params (New%20Current%20Health :type Float%20%28single-precision%29))
  (return 0.0))