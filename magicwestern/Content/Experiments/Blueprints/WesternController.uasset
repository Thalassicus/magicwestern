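; Player controller for a Western-themed character that turns movement, aim and fire input into interface messages on the possessed pawn.
; Movement requests facing rotation only when neither look nor fire input is active.
; Aim comes from the look axes or, while firing, from the cursor's offset from viewport center, normalized by half the viewport size.
; A Respawn event spawns a new WesternCharacter at a player start and possesses it.
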(event EventBeginPlay
  ;[1 1 1] Initialize
  (Variables|Default|SetbShowMouseCursor true))

(event EventRespawn
  ;[1 1 1] Respawn
  (bind _returnvalue (Game|SpawnActorfromClass "/Game/Experiments/Blueprints/WesternCharacter.WesternCharacter_C" (Transformation|GetActorTransform (Class|GameMode|FindPlayerStart (Game|GetGameMode) self)) false 0 0))
  (Pawn|Possess _returnvalue))

(event Input|ActionEvents|InputActionFirePrimaryAction
  (bind _returnvalue (Pawn|GetControlledPawn))
  (bind (_locationx _locationy _returnvalue_2) (Game|Player|GetMousePosition))
  (bind _returnvalue_3 (Viewport|GetViewportSize))
  (bind _returnvalue_4 (/ _returnvalue_3 2.0))
  (bind (_x _y) (Math|Vector2D|BreakVector2D _returnvalue_4))
  ;[1 1 1] Attack
  (:Pressed
    (Class|BPIWesternCharacter|PrimaryAttack(Message) _returnvalue false)
    (Development|PrintString "Firing!")
    ;[1 1 1] Mouse Aiming
    (if (and (!= (stale Input|AxisEvents|InputAxisFirePrimary AxisValue) 0.0) _returnvalue_2)
      (Class|BPIWesternCharacter|Aim(Message) (Pawn|GetControlledPawn) (Math|Vector|MakeVector (/ (- _locationx _x) _x) (/ (- _locationy _y) _y) 0.0))))
  (:Released
    (Class|BPIWesternCharacter|StopPrimaryAttack(Message) _returnvalue)
    (Development|PrintString "Stopped firing!")))

(event Input|AxisEvents|InputAxisLookForward
  (params (AxisValue :type Float%20%28single-precision%29))
  (bind _returnvalue (Input|AxisValues|GetLookForward))
  (bind _returnvalue_2 (Input|AxisValues|GetLookRight))
  ;[1 1 1] Rotation
  (if (not (and (== _returnvalue 0.0) (== _returnvalue_2 0.0)))
    (Class|BPIWesternCharacter|Aim(Message) (Pawn|GetControlledPawn) (Math|Vector|MakeVector _returnvalue_2 _returnvalue 0.0))))

(event Input|AxisEvents|InputAxisLookRight
  (params (AxisValue :type Float%20%28single-precision%29))
  (bind _returnvalue (Input|AxisValues|GetLookForward))
  (bind _returnvalue_2 (Input|AxisValues|GetLookRight))
  ;[1 1 1] Rotation
  (if (not (and (== _returnvalue 0.0) (== _returnvalue_2 0.0)))
    (Class|BPIWesternCharacter|Aim(Message) (Pawn|GetControlledPawn) (Math|Vector|MakeVector _returnvalue_2 _returnvalue 0.0))))

(event Input|AxisEvents|InputAxisFirePrimary
  (params (AxisValue :type Float%20%28single-precision%29))
  (bind (_locationx _locationy _returnvalue) (Game|Player|GetMousePosition))
  (bind _returnvalue_2 (Viewport|GetViewportSize))
  (bind _returnvalue_3 (/ _returnvalue_2 2.0))
  (bind (_x _y) (Math|Vector2D|BreakVector2D _returnvalue_3))
  ;[1 1 1] Mouse Aiming
  (if (and (!= AxisValue 0.0) _returnvalue)
    (Class|BPIWesternCharacter|Aim(Message) (Pawn|GetControlledPawn) (Math|Vector|MakeVector (/ (- _locationx _x) _x) (/ (- _locationy _y) _y) 0.0))))

(event Input|AxisEvents|InputAxisMoveForward
  (params (AxisValue :type Float%20%28single-precision%29))
  (bind _returnvalue (Input|AxisValues|GetMoveForward))
  (bind _returnvalue_2 (Input|AxisValues|GetMoveRight))
  ;[1 1 1] Movement
  (if (not (and (== _returnvalue 0.0) (== _returnvalue_2 0.0)))
    (Class|BPIWesternCharacter|Move(Message) (Pawn|GetControlledPawn) (Math|Vector|MakeVector _returnvalue _returnvalue_2 0.0) (and (== (Input|AxisValues|GetFirePrimary) 0.0) (and (== (Input|AxisValues|GetLookForward) 0.0) (== (Input|AxisValues|GetLookRight) 0.0))))))

(event Input|AxisEvents|InputAxisMoveRight
  (params (AxisValue :type Float%20%28single-precision%29))
  (bind _returnvalue (Input|AxisValues|GetMoveForward))
  (bind _returnvalue_2 (Input|AxisValues|GetMoveRight))
  ;[1 1 1] Movement
  (if (not (and (== _returnvalue 0.0) (== _returnvalue_2 0.0)))
    (Class|BPIWesternCharacter|Move(Message) (Pawn|GetControlledPawn) (Math|Vector|MakeVector _returnvalue _returnvalue_2 0.0) (and (== (Input|AxisValues|GetFirePrimary) 0.0) (and (== (Input|AxisValues|GetLookForward) 0.0) (== (Input|AxisValues|GetLookRight) 0.0))))))

(fn ConstructionScript)