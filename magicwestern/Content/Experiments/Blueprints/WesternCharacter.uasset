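; Western shooter character with camera-relative movement and independent aiming, in a twin-stick style.
; Move and Aim events flatten input onto CameraArm axes and yaw the mesh toward movement or aim direction.
; Primary attack fires immediately, then loops ShootGun on a timer, damaging every multi-line-trace hit along the aim direction.
; Tick draws debug direction lines; the fall-death respawn and RefireWeapon timer logic are unconnected.
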(event Custom|RefireWeapon
  ;[1 1 1] Primary Attack
  (Weapon|ShootGun)
  (Variables|Weapon|SetCanShoot false))

(event EventMove
  (params (Direction :type Vector) (DoRotation :type Boolean))
  (bind _returnvalue (Transformation|GetActorLocation))
  ;[1 1 1] Movement (+x = forward)
  (bind _local_direction (Utility|Localize Direction (Variables|Default|GetCameraArm)))
  (bind _output_get (Variables|Movement|SetMoveDirection _local_direction))
  (Pawn|Input|AddMovementInput _output_get (* (Variables|Movement|GetMoveSpeed) (Math|Vector|VectorLength Direction)) false)
  (if DoRotation
    (Variables|Utility|SetCanMovementRotate DoRotation)
    ;[1 1 1] Aim (+x = forward)
    (Transformation|SetWorldRotation (Variables|Character|GetMesh) (Class|KismetMathLibrary|MakeRot 0.0 (.Yaw (Class|KismetMathLibrary|BreakRot (Math|Rotator|FindLookatRotation _returnvalue (+ (Math|Vector|SelectVector (Math|Vector|MakeVector (.Y (Math|Vector|BreakVector (Variables|Movement|GetMoveDirection))) (* (.X (Math|Vector|BreakVector (Variables|Movement|GetMoveDirection))) -1.0) 0.0) (stale EventAim _output_get) (Variables|Utility|GetCanMovementRotate)) _returnvalue)))) 0.0) false)))

(event EventAim
  (params (Direction :type Vector))
  (bind _returnvalue (Transformation|GetActorLocation))
  (bind _movedirection (Variables|Movement|GetMoveDirection))
  (bind (_x _y) (Math|Vector|BreakVector _movedirection))
  ;[1 1 1] Aim (+x = forward)
  (bind _local_direction (Utility|Localize Direction (Variables|Default|GetCameraArm)))
  (bind _output_get (Variables|Aim|SetTargetDirection _local_direction))
  (Variables|Utility|SetCanMovementRotate false)
  (Transformation|SetWorldRotation (Variables|Character|GetMesh) (Class|KismetMathLibrary|MakeRot 0.0 (.Yaw (Class|KismetMathLibrary|BreakRot (Math|Rotator|FindLookatRotation _returnvalue (+ (Math|Vector|SelectVector (Math|Vector|MakeVector _y (* _x -1.0) 0.0) _output_get (Variables|Utility|GetCanMovementRotate)) _returnvalue)))) 0.0) false))

(event EventPrimaryAttack
  (params (IsShooting :type Boolean))
  ;[1 1 1] Primary Attack
  (Variables|Weapon|SetIsShooting true)
  (Weapon|ShootGun)
  (Utilities|Time|SetTimerbyFunctionName 0 "ShootGun" (Variables|Weapon|GetFireRate) true))

(event EventStopPrimaryAttack
  ;[1 1 1] Primary Attack
  (Variables|Weapon|SetIsShooting false)
  (Class|KismetSystemLibrary|PauseTimer 0 "ShootGun")
  (Utilities|Time|ClearTimerbyFunctionName 0 "ShootGun"))

(event EventTick
  (params (DeltaSeconds :type Float%20%28single-precision%29))
  (bind _targetdirection (Variables|Aim|GetTargetDirection))
  (bind _arrow1 (Variables|Default|GetArrow1))
  (bind _returnvalue (Math|Vector|RotateVectorAroundAxis _targetdirection 9e+01 "0,0.000000,1.000000"))
  (bind _relativelocation (Variables|/Script/Engine.SceneComponent|GetRelativeLocation _arrow1))
  ;[1 1 1] Actor Death
  ;[1 1 1] Debug
  (Rendering|Debug|FlushPersistentDebugLines)
  (Utility|DrawLine (Variables|Movement|GetMoveDirection) "(R=1.000000,G=0.000000,B=0.000000,A=1.000000)" 1.0 _relativelocation 128.0)
  (if (Variables|Weapon|GetIsShooting)
    (Utility|DrawLine _returnvalue "(R=0.000000,G=0.000000,B=1.000000,A=1.000000)" 1.0 _relativelocation 128.0)
    (else
      (Utility|DrawLine _returnvalue "(R=1.000000,G=0.500000,B=0.000000,A=1.000000)" 1.0 _relativelocation 128.0))))

(fn ConstructionScript)

(fn Localize
  (params (Direction :type Vector) (Local%20Target :type Scene%20Component%20Object%20Reference))
  (bind (_x _y) (Math|Vector|BreakVector Direction))
  (bind _returnvalue (Math|Vector|GetForwardVector Local%20Target))
  (bind _returnvalue_2 (Math|Vector|GetRightVector Local%20Target))
  (bind (_x_2 _y_2) (Math|Vector|BreakVector _returnvalue_2))
  (bind (_x_3 _y_3) (Math|Vector|BreakVector _returnvalue))
  (return (Math|Vector|Normalize (+ (* (Math|Vector|Normalize (Math|Vector|MakeVector _x_3 _y_3 0.0)) _x) (* (Math|Vector|Normalize (Math|Vector|MakeVector _x_2 _y_2 0.0)) _y)))))

(fn DrawLine
  (params (Direction :type Vector) (Color :type Linear%20Color%20Structure) (Duration :type Float%20%28single-precision%29) (Offset :type Vector) (Length :type Float%20%28single-precision%29))
  (bind _returnvalue (Transformation|GetActorLocation))
  (bind _returnvalue_2 (+ Offset _returnvalue))
  (bind _asplayer_controller (Utilities|Casting|CastToPlayerController (Pawn|GetController))
    (:then
      (Rendering|Debug|DrawDebugLine (HUD|GetHUD _asplayer_controller) _returnvalue_2 (+ _returnvalue_2 (* (Math|Vector|Normalize Direction) Length)) Color Duration 2.0))
    (:CastFailed
      (Development|PrintString "FAILED!"))))

(fn ShootGun
  (bind _returnvalue (Transformation|GetActorLocation))
  (bind (_outhits _returnvalue_2) (Class|KismetSystemLibrary|LineTraceMultiNEW _returnvalue (+ _returnvalue (* (Math|Vector|Normalize (Variables|Aim|GetTargetDirection)) 9999.0)) "TraceTypeQuery1" false 0 "None" true))
  (if _returnvalue_2
    (for _array_element _outhits
      (Game|Damage|ApplyDamage (.HitActor (Collision|BreakHitResult _array_element)) 1.0 (Game|GetInstigatorController) self))))