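; Target dummy actor that plays a one-shot hit animation on its mesh whenever it takes any damage.
; A separate DrawLine helper draws a timed debug line from the actor's location plus an offset along a normalized direction.
; The helper only draws when the dummy's controller is a PlayerController, using that controller's HUD as world context, and nothing in this file calls it.
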(event Game|Damage|EventAnyDamage
  (params (Damage :type Float%20%28single-precision%29) (DamageType :type Damage%20Type%20Object%20Reference) (InstigatedBy :type Controller%20Object%20Reference) (DamageCauser :type Actor%20Object%20Reference))
  (Components|Animation|PlayAnimation (Variables|Character|GetMesh) "/Game/Experiments/Objects/TargetDummy/TargetDummy_Hit.TargetDummy_Hit" false))

(fn ConstructionScript)

(fn DrawLine
  (params (Direction :type Vector) (Color :type Linear%20Color%20Structure) (Duration :type Float%20%28single-precision%29) (Offset :type Vector) (Length :type Float%20%28single-precision%29))
  (bind _returnvalue (Transformation|GetActorLocation))
  (bind _returnvalue_2 (+ Offset _returnvalue))
  (bind _asplayer_controller (Utilities|Casting|CastToPlayerController (Pawn|GetController)))
  (Rendering|Debug|DrawDebugLine (HUD|GetHUD _asplayer_controller) _returnvalue_2 (+ _returnvalue_2 (* (Math|Vector|Normalize Direction) Length)) Color Duration 2.0))