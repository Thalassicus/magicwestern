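; Dev target dummy that holds a handgun, turns to face nearby players and can be damaged until dead.
; Each tick it yaws its mesh toward the closest WesternCharacter within range and sets HasTarget, with no firing logic.
; Damage lowers health and plays a hit animation, or at zero loops a death animation, disables capsule collision and stops tracking.
; DrawLine is a debug helper that nothing here calls.
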(event Game|Damage|EventAnyDamage
  (params (Damage :type Float%20%28single-precision%29) (DamageType :type Damage%20Type%20Object%20Reference) (InstigatedBy :type Controller%20Object%20Reference) (DamageCauser :type Actor%20Object%20Reference))
  (bind _mesh (Variables|Character|GetMesh))
  ;[1 1 1] Take Damage
  (if (not (Variables|Health|GetIsDead))
    (bind _output_get (Variables|Health|SetHealth (Math|Float|Clamp(Float) (- (Variables|Health|GetHealth) Damage) 0.0 (Variables|Health|GetMaxHealth))))
    (if (> _output_get 0.0)
      (Components|Animation|PlayAnimation _mesh "/Game/Experiments/Objects/dev_TargetDummy/TargetDummy_Hit.TargetDummy_Hit" false)
      (else
        (Components|Animation|PlayAnimation _mesh "/Game/Experiments/Objects/dev_TargetDummy/TargetDummy_DeathIdle.TargetDummy_DeathIdle" true)
        (Variables|Health|SetIsDead true)
        (Collision|SetCollisionEnabled (Variables|Collision|GetCapsuleComponent) "NoCollision")))))

(event EventBeginPlay
  ;[1 1 1] Initialize
  (Variables|Health|SetHealth (Variables|Health|GetMaxHealth))
  (Components|Animation|SetAnimation (Variables|Character|GetMesh) "/Game/Experiments/Objects/dev_TargetDummy/TargetDummy_AimIdle.TargetDummy_AimIdle")
  (Class|SceneComponent|Attachto (Variables|Default|GetBP_dev_HandGun) (Variables|Character|GetMesh) "B_RightHandSocket" "SnapToTarget" true))

(event EventTick
  (params (DeltaSeconds :type Float%20%28single-precision%29))
  (bind _capsulecomponent (Variables|Collision|GetCapsuleComponent))
  (bind _returnvalue (Transformation|GetWorldLocation _capsulecomponent))
  ;[1 1 1] Look at closest player
  (if (not (Variables|Health|GetIsDead))
    (bind (_found_target _target_position) (CallFunction|FindClosestPlayer _returnvalue))
    (if _found_target
      (Transformation|SetWorldRotation (Variables|Character|GetMesh) (Class|KismetMathLibrary|MakeRot 0.0 (.Yaw (Class|KismetMathLibrary|BreakRot (Math|Rotator|FindLookatRotation _returnvalue _target_position))) 0.0) false)
      (Variables|Weapon|SetHas%20Target true)
      (else
        (Variables|Weapon|SetHas%20Target false)))))

(fn ConstructionScript)

(fn DrawLine
  (params (Direction :type Vector) (Color :type Linear%20Color%20Structure) (Duration :type Float%20%28single-precision%29) (Offset :type Vector) (Length :type Float%20%28single-precision%29))
  (bind _returnvalue (Transformation|GetActorLocation))
  (bind _returnvalue_2 (+ Offset _returnvalue))
  (bind _asplayer_controller (Utilities|Casting|CastToPlayerController (Pawn|GetController)))
  (Rendering|Debug|DrawDebugLine (HUD|GetHUD _asplayer_controller) _returnvalue_2 (+ _returnvalue_2 (* (Math|Vector|Normalize Direction) Length)) Color Duration 2.0))

(fn FindClosestPlayer
  (params (Start%20Position :type Vector))
  (LocalVariables|SetStartPosition Start%20Position)
  (bind _outactors (Actor|GetAllActorsOfClass "/Game/Experiments/Objects/WesternCharacter_Topdown/WesternCharacter.WesternCharacter_C"))
  (for _index (range 0 (Utilities|Array|Length _outactors))
    (if (and (< (Math|Vector|VectorLength (- (LocalVariables|GetStartPosition) (Transformation|GetActorLocation (Utilities|Array|Get(acopy) _outactors _index)))) (LocalVariables|GetClosestDistance)) (< (Math|Vector|VectorLength (- (LocalVariables|GetStartPosition) (Transformation|GetActorLocation (Utilities|Array|Get(acopy) _outactors _index)))) (Variables|Weapon|GetMaximum%20Target%20Distance)))
      (LocalVariables|SetClosestDistance (Math|Vector|VectorLength (- (LocalVariables|GetStartPosition) (Transformation|GetActorLocation (Utilities|Array|Get(acopy) _outactors _index)))))
      (LocalVariables|SetClosestPosition (Transformation|GetActorLocation (Utilities|Array|Get(acopy) _outactors _index)))))
  (return (Math|Vector|NotEqual(Vector) (LocalVariables|GetClosestPosition) "0, 0, 0" 0.0001) (LocalVariables|GetClosestPosition)))