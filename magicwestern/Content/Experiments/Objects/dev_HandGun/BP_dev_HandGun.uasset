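; Development handgun Blueprint that fires penetrating hitscan shots, with a stubbed reload.
; Timers delay each shot and reload, using flags to block re-entry and stop events to cancel.
; Shoot plays a sound and multi-traces Pawns from SourceObject along TargetDirection rotated 90 degrees, with persistent debug drawing.
; BPI_BulletBlocker targets return the remaining damage; other hits take that damage, then halve it for the next.
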(event Custom|Reload%20Helper
  ;[1 1 1] Reload
  (CallFunction|Reload)
  (Variables|Weapon|SetCan%20Reload true))

(event Custom|Shoot%20Helper
  ;[1 1 1] Shoot
  (CallFunction|Shoot)
  (Variables|Weapon|SetCan%20Shoot true))

(event EventDoShoot
  ;[1 1 1] Shoot
  (bind _can_shoot (CallFunction|GetCanShoot))
  (if _can_shoot
    (Variables|Weapon|SetCan%20Shoot false)
    (Utilities|Time|SetTimerbyEvent (delegate Custom|Shoot%20Helper) (Variables|Weapon|GetFire%20Rate))))

(event EventDoReload
  ;[1 1 1] Reload
  (if (Variables|Weapon|GetCan%20Reload)
    (Variables|Weapon|SetCan%20Reload false)
    (Utilities|Time|SetTimerbyEvent (delegate Custom|Reload%20Helper) (Variables|Weapon|GetReload%20Rate))))

(event EventStopShoot
  ;[1 1 1] Shoot
  (Variables|Weapon|SetCan%20Shoot true)
  (Class|KismetSystemLibrary|PauseTimerDelegate (delegate Custom|Shoot%20Helper))
  (Class|KismetSystemLibrary|ClearTimerDelegate (delegate Custom|Shoot%20Helper)))

(event EventStopReload
  ;[1 1 1] Reload
  (Variables|Weapon|SetCan%20Reload true)
  (Class|KismetSystemLibrary|PauseTimerDelegate (delegate Custom|Reload%20Helper))
  (Class|KismetSystemLibrary|ClearTimerDelegate (delegate Custom|Reload%20Helper)))

(fn ConstructionScript)

(fn GetCanShoot
  (return (and (Variables|Weapon|GetCan%20Shoot) (Variables|Weapon|GetCan%20Reload))))

(fn Reload
  (return false))

(fn Shoot
  (bind _source_object (Variables|Weapon|GetSource%20Object))
  (bind _returnvalue (Transformation|GetActorLocation _source_object))
  (Class|GameplayStatics|PlaySoundAttached "/Game/TwinStickBP/Audio/TemplateTSS_WeaponFire.TemplateTSS_WeaponFire" (Variables|Default|Getdev_HandGunMesh))
  (LocalVariables|SetRemaining%20Damage (Variables|Weapon|GetDamage))
  (bind (_outhits _returnvalue_2) (Class|KismetSystemLibrary|LineTraceMultiforObjects _returnvalue (+ _returnvalue (* (Math|Vector|RotateVectorAroundAxis (Variables|Weapon|GetTarget%20Direction) 9e+01 "0,0.000000,1.000000") 9999.0)) (Utilities|Array|MakeArray "ObjectTypeQuery3") false 0 "Persistent" true))
  (if _returnvalue_2
    (for _array_element _outhits
      (if (Utilities|DoesObjectImplementInterface (.HitActor (Collision|BreakHitResult _array_element)) "/Game/Experiments/Blueprints/Interfaces/BPI_BulletBlocker.BPI_BulletBlocker_C")
        (bind _remaining_damage (Class|BPIBulletBlocker|GetPenetrationDamage(Message) (.HitActor (Collision|BreakHitResult _array_element)) 0 (LocalVariables|GetRemaining%20Damage)))
        (LocalVariables|SetRemaining%20Damage _remaining_damage)
        (LocalVariables|SetHas%20Done%20Damage true)
        (else
          (LocalVariables|SetHas%20Done%20Damage false)))
      (if (and (> (LocalVariables|GetRemaining%20Damage) 0.0) (not (LocalVariables|GetHas%20Done%20Damage)))
        (Game|Damage|ApplyDamage (.HitActor (Collision|BreakHitResult _array_element)) (LocalVariables|GetRemaining%20Damage) 0 0)
        (if (not (LocalVariables|GetHas%20Done%20Damage))
          (LocalVariables|SetRemaining%20Damage (/ (LocalVariables|GetRemaining%20Damage) 2.0))))))
  (return true))