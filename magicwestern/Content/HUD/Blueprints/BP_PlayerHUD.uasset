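; Player HUD Blueprint that draws a labeled health bar on screen.
; The construction script creates a dynamic instance of the HUD_Healthbar material.
; Each DrawHUD polls the player pawn's BP_Health component, feeds the current-to-maximum health ratio into the material, then draws it at fixed screen coordinates.
; Bar width scales with maximum health, with a minimum size, while the material parameter conveys the fill.
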(event EventDrawHUD
  (params (SizeX :type Integer) (SizeY :type Integer))
  (Variables|Default|SetScreen%20Dimensions (Math|Vector2D|MakeVector2D (Math|Conversions|ToFloat(Integer) SizeX) (Math|Conversions|ToFloat(Integer) SizeY)))
  (bind (_current_health _maximum_health) (Class|BPIHealth|GetHealth(Message) (Utilities|Array|Get(acopy) (Actor|GetComponentsByClass (Game|Player|GetPlayerPawn 0) "/Game/Blueprints/ActorBasics/BP_Health.BP_Health_C"))))
  (Rendering|Material|SetScalarParameterValue (Variables|Default|GetHealth%20bar) "Health percentage" (/ _current_health _maximum_health) :!class /Script/Engine.MaterialInstanceDynamic) ; Updates a parameter in the health bar material
  (HUD|DrawText "Health:" (Variables|Default|GetWhite) 5e+01 8e+01 "/Engine/EngineFonts/RobotoDistanceField.RobotoDistanceField" 1.0 false) ; Draw "Health:" text at the specified screen coordinates
  (Class|HUD|DrawMaterialSimple (Variables|Default|GetHealth%20bar) 125.0 8e+01 (Math|Float|Max(Float) (* _maximum_health 2.0) 2e+01) 25.0 1.0 false))

(fn ConstructionScript
  (bind _returnvalue (Rendering|Material|CreateDynamicMaterialInstance "/Game/HUD/Materials/HUD_Healthbar.HUD_Healthbar" :!class /Script/Engine.KismetMaterialLibrary)) ; Create a dunamic material instance of a health bar material
  (Variables|Default|SetHealth%20bar _returnvalue))